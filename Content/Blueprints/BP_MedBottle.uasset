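; BP_MedBottle is a hoverable penicillin bottle actor that brings up the Game_Over screen when its click event fires.
; Cursor overlap sets a hover flag, which Tick uses to show the label widget and smoothly raise or lower the mesh.
; Tick also yaw-billboards the label toward the player camera and rewrites its text every frame.
; After game over, releasing Space opens Level_1 and removes the screen.
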(event EventBeginPlay
  (Variables|Default|SetDefaultPos (Variables|/Script/Engine.SceneComponent|GetRelativeLocation (Variables|Debug|GetStaticMeshComponent))))

(event EventTick
  (params (DeltaSeconds :type Float%20%28single-precision%29))
  (bind _widget (Variables|Default|GetWidget))
  (bind _defaultpos (Variables|Default|GetDefaultPos))
  (bind _widget_2 (Variables|Default|GetWidget))
  (bind _staticmeshcomponent (Variables|Debug|GetStaticMeshComponent))
  (bind _returnvalue (Transformation|GetWorldRotation _widget_2))
  (bind _relativelocation (Variables|/Script/Engine.SceneComponent|GetRelativeLocation _staticmeshcomponent))
  (Utilities|FlowControl|Sequence
    (:then_0
      (if (Variables|Default|GetisHovering)
        (Rendering|SetVisibility _widget true false)
        (Transformation|SetRelativeLocation (Variables|Debug|GetStaticMeshComponent) (Math|Interpolation|VInterpTo _relativelocation (+ _defaultpos "0, 0,2.000000") DeltaSeconds 5.0) false false)
        (else
          (Rendering|SetVisibility _widget false false)
          (Transformation|SetRelativeLocation (Variables|Debug|GetStaticMeshComponent) (Math|Interpolation|VInterpTo _relativelocation _defaultpos DeltaSeconds 5.0) false false))))
    (:then_1
      (Transformation|SetWorldRotation _widget_2 (Math|Rotator|MakeRotator (.roll _returnvalue) (.pitch _returnvalue) (.yaw (Math|Rotator|FindLookatRotation (Transformation|GetWorldLocation (Variables|Default|GetWidget)) (Transformation|GetWorldLocation (Variables|/Script/Engine.PlayerCameraManager|GetTransformComponent (Game|GetPlayerCameraManager 0)))))) false false)
      (bind _asmeds_widget (Utilities|Casting|CastToMeds_Widget (UserInterface|GetUserWidgetObject (Variables|Default|GetWidget))))
      (Rendering|Components|TextRender|SetText (Variables|/Game/UI/Meds_Widget.Meds_Widget_C|GettxtMediLbl _asmeds_widget) "PENICILLIN 
(ANTI-BIOTIC)"))))

(event MouseInput|EventActorBeginCursorOver
  (Variables|Default|SetisHovering true))

(event MouseInput|EventActorEndCursorOver
  (Variables|Default|SetisHovering false))

(event EventIsClickedon
  (bind _returnvalue (UserInterface|CreateWidget "/Game/UI/Game_Over.Game_Over_C" (Game|GetPlayerController 0)))
  (UserInterface|Viewport|AddtoViewport _returnvalue 0)
  (Variables|Default|SetEnd_Screen true)
  (Input|EnableInput (Game|GetPlayerController 0)))

(event Input|KeyboardEvents|SpaceBar
  (params (Key :type Key%20Structure))
  (:Released
    (if (Variables|Default|GetEnd_Screen)
      (Game|OpenLevel(byName) "Level_1")
      (Widget|RemovefromParent (stale EventIsClickedon _returnvalue)))))

(fn ConstructionScript)