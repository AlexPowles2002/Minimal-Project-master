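; BP_Tut is a world-placed text prompt, apparently for tutorials, that displays a WBP_Tut widget and keeps it turned toward the player camera.
; Every Tick it sets the Pivot's world rotation to look at the camera manager's location, adding an Offset to the yaw.
; Helper functions set the widget's TutText, toggle in-game visibility for the whole component hierarchy, and move the actor.
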(event EventBeginPlay)

(event Collision|EventActorBeginOverlap
  (params (OtherActor :type Actor%20Object%20Reference)))

(event EventTick
  (params (DeltaSeconds :type Float%20%28single-precision%29))
  (bind _returnvalue (Game|GetPlayerCameraManager 0))
  (bind _pivot (Variables|Default|Getpivot))
  (bind _returnvalue_2 (Transformation|GetActorLocation _returnvalue))
  (bind _returnvalue_3 (Transformation|GetWorldLocation _pivot))
  (bind _returnvalue_4 (Math|Rotator|FindLookatRotation _returnvalue_3 _returnvalue_2))
  (bind _returnvalue_5 (Math|Transform|MakeTransform _returnvalue_3 _returnvalue_4))
  (Transformation|SetWorldRotation (Variables|Default|Getpivot) (Math|Rotator|MakeRotator (.roll (.rotation _returnvalue_5)) (.pitch (.rotation _returnvalue_5)) (+ (Variables|Default|Getoffset) (.yaw (.rotation _returnvalue_5)))) false false))

(fn ConstructionScript)

(fn SetText
  (params (InText :type Text))
  (Rendering|Components|TextRender|SetText (Variables|/Game/Blueprints/WBP_Tut.WBP_Tut_C|GetTutText (.AsWBP%20Tut (Utilities|Casting|CastToWBP_Tut (UserInterface|GetUserWidgetObject (Variables|Default|GetWidget))))) InText))

(fn SetVisibility
  (params (NewHidden :type Boolean))
  (Development|SetHiddeninGame (Variables|Default|GetDefaultSceneRoot) NewHidden true))

(fn SetLoc
  (params (NewLocation :type Vector))
  (Transformation|SetActorLocation NewLocation false false))