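; BP_Radio is a radio that plays and pauses its audio when clicked.
; A click while StopRepeat is set clears the flag, starts the audio from the beginning and binds its finished event, which sets the flag again.
; Other clicks run a FlipFlop that alternates unpause and pause, starting with unpause and never reset on replay.
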(event Custom|OnAudioFinished_Event_0
  (Variables|Default|SetStop_Repeat true))

(event EventIsClickedon
  (bind _audio (Variables|Default|GetAudio))
  (if (Variables|Default|GetStop_Repeat)
    (Variables|Default|SetStop_Repeat false)
    (Audio|Components|Audio|Play _audio 0.0)
    (EventDispatchers|AssignOnAudioFinished _audio (delegate Custom|OnAudioFinished_Event_0))
    (else
      (Utilities|FlowControl|FlipFlop
        (:A
          (Class|AudioComponent|SetPaused _audio false))
        (:B
          (Class|AudioComponent|SetPaused _audio true))))))

(fn ConstructionScript)